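; Game mode that tracks arena progress and shows the end-of-game screens.
; On BeginPlay it counts every BP_ArenaTrigger in the level and binds to each one's OnArenaCleared event, triggering victory once all are cleared.
; ShowVictory and ShowDefeat wait briefly, then add their widget, show the cursor and switch to UI-only input.
; Nothing in this Blueprint calls ShowDefeat.
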(event Custom|ShowVictory
  (bind _returnvalue (Game|GetPlayerController 0))
  (Utilities|FlowControl|Delay 3.0)
  (bind _returnvalue_2 (UserInterface|CreateWidget "/Game/_Project/02_UI/Widgets/WBP_Victory.WBP_Victory_C" _returnvalue))
  (UserInterface|Viewport|AddtoViewport _returnvalue_2 0)
  (Variables|/Script/Engine.PlayerController|SetbShowMouseCursor _returnvalue true)
  (Input|SetInputModeUIOnly _returnvalue _returnvalue_2 "DoNotLock" false))

(event Custom|ShowDefeat
  (bind _returnvalue (Game|GetPlayerController 0))
  (Utilities|FlowControl|Delay 3.0)
  (bind _returnvalue_2 (UserInterface|CreateWidget "/Game/_Project/02_UI/Widgets/WBP_Defeat.WBP_Defeat_C" _returnvalue))
  (UserInterface|Viewport|AddtoViewport _returnvalue_2 0)
  (Variables|/Script/Engine.PlayerController|SetbShowMouseCursor _returnvalue true)
  (Input|SetInputModeUIOnly _returnvalue _returnvalue_2 "DoNotLock" false))

(event Custom|GM_OnArenaCleared
  (bind _output_get (Variables|Default|SetClearedArenas (+ (Variables|Default|GetClearedArenas) 1)))
  (if (>= _output_get (Variables|Default|GetTotalArenas))
    (CallFunction|ShowVictory)))

(event EventBeginPlay
  (bind _outactors (Actor|GetAllActorsOfClass "/Game/_Project/01_Blueprints/World/BP_ArenaTrigger.BP_ArenaTrigger_C"))
  (Variables|Default|SetTotalArenas (Utilities|Array|Length _outactors))
  (Variables|Default|SetClearedArenas 0)
  (for _array_element _outactors
    (EventDispatchers|BindEventtoOnArenaCleared _array_element (delegate Custom|GM_OnArenaCleared))))

(event EventTick
  (params (DeltaSeconds :type Float%20%28single-precision%29)))

(fn ConstructionScript)