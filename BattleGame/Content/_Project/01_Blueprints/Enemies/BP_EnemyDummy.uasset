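; BP_EnemyDummy is an enemy character dummy that takes damage and can die.
; Any damage reduces HP with debug prints, and at zero or below it sets IsDead and fires the OnDied dispatcher.
; Only BeginPlay applies the ragdoll (movement and capsule collision off, mesh physics on), and only if IsDead is already set, also firing OnDied.
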(event EventBeginPlay
  (if (Variables|Default|GetbIsDead)
    (Default|CallOnDied)
    (Pawn|Components|CharacterMovement|DisableMovement (Variables|Character|GetCharacterMovement))
    (Collision|SetCollisionEnabled (Variables|Collision|GetCapsuleComponent) "NoCollision")
    (Physics|SetSimulatePhysics (Variables|Character|GetMesh) true)))

(event Collision|EventActorBeginOverlap
  (params (OtherActor :type Actor%20Object%20Reference)))

(event EventTick
  (params (DeltaSeconds :type Float%20%28single-precision%29)))

(event Game|Damage|EventAnyDamage
  (params (Damage :type Float%20%28single-precision%29) (DamageType :type Damage%20Type%20Object%20Reference) (InstigatedBy :type Controller%20Object%20Reference) (DamageCauser :type Actor%20Object%20Reference))
  (Development|PrintString (Utilities|String|Append "Damage " (Utilities|String|ToString(Float) Damage)))
  (bind _output_get (Variables|Default|SetHP (- (Variables|Default|GetHP) Damage)))
  (Development|PrintString (Utilities|String|Append "HP " (Utilities|String|ToString(Float) _output_get)))
  (if (<= _output_get 0.0)
    (Variables|Default|SetbIsDead true)
    (Default|CallOnDied)))

(fn ConstructionScript)