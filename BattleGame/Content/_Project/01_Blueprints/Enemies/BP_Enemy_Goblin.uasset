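; Goblin enemy Blueprint that varies its attacks between a normal swing and an occasional, stronger jump attack.
; SelectGoblinAttack counts attacks and triggers a jump once the counter reaches a random threshold set on BeginPlay and re-rolled after each jump.
; Each selection sets the montage and hit delay, plus a jump flag, with a raised damage multiplier for jumps.
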(event EventBeginPlay
  (|CallParentFunction)
  (Variables|Default|SetNextJumpAt (Math|Random|RandomIntegerinRange 2 6)))

(event Collision|EventActorBeginOverlap
  (params (OtherActor :type Actor%20Object%20Reference))
  (|CallParentFunction OtherActor) ; This node is disabled and will not be called.\nDrag off pins to build functionality.
)

(event EventTick
  (params (DeltaSeconds :type Float%20%28single-precision%29))
  (|CallParentFunction DeltaSeconds) ; This node is disabled and will not be called.\nDrag off pins to build functionality.
)

(fn ConstructionScript
  (|CallParentFunction))

(fn SelectGoblinAttack
  (bind _output_get (Variables|Default|SetAttackCounter (+ (Variables|Default|GetAttackCounter) 1)))
  (if (>= _output_get (Variables|Default|GetNextJumpAt))
    (Variables|Default|SetAttackCounter 0)
    (Variables|Default|SetNextJumpAt (Math|Random|RandomIntegerinRange 2 6))
    (Variables|Default|SetAttackMontage (Variables|Default|GetAttackMontage_Jump))
    (Variables|Default|SetAttackHitDelay (Variables|Default|GetHitDelay_Jump))
    (Variables|Default|SetJumpDamageMultiplier 2.0)
    (Variables|Default|SetbNextAttackIsJump true)
    (else
      (Variables|Default|SetAttackMontage (Variables|Default|GetAttackMontage_Normal))
      (Variables|Default|SetAttackHitDelay (Variables|Default|GetHitDelay_Normal))
      (Variables|Default|SetbNextAttackIsJump false))))