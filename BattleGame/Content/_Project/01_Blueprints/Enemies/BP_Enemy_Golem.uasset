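; BP_Enemy_Golem is a golem enemy that mixes default attacks with periodic area-of-effect attacks.
; SelectGolemAttack counts attacks and, on reaching a randomized threshold, picks the AOE attack, resets the counter and rerolls the threshold.
; Each selection sets the montage, hit delay, damage (multiplied for AOE) and an AOE flag, without executing the attack itself.
; BeginPlay calls the parent and rolls the first threshold.
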(event EventBeginPlay
  (|CallParentFunction)
  (Variables|Default|SetNextAOEAt (Math|Random|RandomIntegerinRange 2 6)))

(event Collision|EventActorBeginOverlap
  (params (OtherActor :type Actor%20Object%20Reference))
  (|CallParentFunction OtherActor) ; This node is disabled and will not be called.\nDrag off pins to build functionality.
)

(event EventTick
  (params (DeltaSeconds :type Float%20%28single-precision%29))
  (|CallParentFunction DeltaSeconds) ; This node is disabled and will not be called.\nDrag off pins to build functionality.
)

(fn ConstructionScript
  (|CallParentFunction))

(fn SelectGolemAttack
  (bind _output_get (Variables|Default|SetAttacckCounter (+ (Variables|Default|GetAttacckCounter) 1)))
  (if (>= _output_get (Variables|Default|GetNextAOEAt))
    (Variables|Default|SetAttacckCounter 0)
    (Variables|Default|SetNextAOEAt (Math|Random|RandomIntegerinRange 2 6))
    (Variables|Default|SetAttackMontage (Variables|Default|GetAOE_Montage))
    (Variables|Default|SetHitDelay (Variables|Default|GetHitDelay_AOE))
    (Variables|Default|SetDamageToApply (* (Variables|Default|GetDamage) (Variables|Default|GetAOE_DamageMultiplier)))
    (Variables|Default|SetbNextAttackAOEGolem true)
    (else
      (Variables|Default|SetAttackMontage (Variables|Default|GetDefault_attack))
      (Variables|Default|SetHitDelay 1.1)
      (Variables|Default|SetDamageToApply (Variables|Default|GetDamage))
      (Variables|Default|SetbNextAttackAOEGolem false))))