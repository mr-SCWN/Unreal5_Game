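; BP_Door is a world door that slides vertically between a closed and an open position.
; BeginPlay caches the mesh's starting relative location as closed and offsets it by OpenHeight on Z for the open position.
; OpenDoor and CloseDoor events set IsOpen and play or reverse a timeline that lerps the mesh between the two, without sweep.
; Nothing in this Blueprint calls those events itself.
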(event Custom|OpenDoor
  (Variables|Default|SetbIsOpen true)
  (bind _alpha (Timeline|TL_DoorMove Play)
    (:Update
      (Transformation|SetRelativeLocation (Variables|Default|GetDoorMesh) (Math|Vector|Lerp(Vector) (Variables|Default|GetClosedLocation) (Variables|Default|GetOpenLocation) _alpha) false false))))

(event Custom|CloseDoor
  (Variables|Default|SetbIsOpen false)
  (bind _alpha (Timeline|TL_DoorMove Reverse)
    (:Update
      (Transformation|SetRelativeLocation (Variables|Default|GetDoorMesh) (Math|Vector|Lerp(Vector) (Variables|Default|GetClosedLocation) (Variables|Default|GetOpenLocation) _alpha) false false))))

(event EventBeginPlay
  (bind _output_get (Variables|Default|SetClosedLocation (Variables|/Script/Engine.SceneComponent|GetRelativeLocation (Variables|Default|GetDoorMesh))))
  (Variables|Default|SetOpenLocation (+ _output_get (Math|Vector|MakeVector 0.0 0.0 (Variables|Default|GetOpenHeight)))))

(event Collision|EventActorBeginOverlap
  (params (OtherActor :type Actor%20Object%20Reference)))

(event EventTick
  (params (DeltaSeconds :type Float%20%28single-precision%29)))

(fn ConstructionScript)