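; BP_LiftTrigger is a one-shot lift trigger that upgrades the player between closing one door and opening another.
; When BP_ThirdPersonCharacter overlaps LiftBox, it closes DoorToClose, waits briefly, then shows WBP_LiftUpgrade with UI-only input and pauses the game.
; It also raises and refills HP and Stamina directly and refreshes the HUD.
; DoorToOpen opens after OpenDelay, a Delay started while paused.
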(event OnComponentBeginOverlap(LiftBox)
  (params (OverlappedComponent :type Primitive%20Component%20Object%20Reference) (OtherActor :type Actor%20Object%20Reference) (OtherComp :type Primitive%20Component%20Object%20Reference) (OtherBodyIndex :type Integer) (bFromSweep :type Boolean) (SweepResult :type Hit%20Result%20Structure%20%28by%20ref%29))
  (bind _returnvalue (Game|GetPlayerController 0))
  (bind _asbp_third_person_character (Utilities|Casting|CastToBP_ThirdPersonCharacter OtherActor))
  (if (not (Variables|Default|GetbTriggered))
    (Variables|Default|SetbTriggered true)
    (Default|CloseDoor (Variables|Default|GetDoorToClose))
    (Utilities|FlowControl|Delay 1.0)
    (bind _returnvalue_2 (UserInterface|CreateWidget "/Game/_Project/02_UI/Widgets/WBP_LiftUpgrade.WBP_LiftUpgrade_C" _returnvalue _asbp_third_person_character))
    (UserInterface|Viewport|AddtoViewport _returnvalue_2 0)
    (Variables|/Script/Engine.PlayerController|SetbShowMouseCursor _returnvalue true)
    (Input|SetInputModeUIOnly _returnvalue _returnvalue_2 "DoNotLock" false)
    (Game|SetGamePaused true)
    (bind _output_get (Variables|/Game/ThirdPerson/Blueprints/BP_ThirdPersonCharacter.BP_ThirdPersonCharacter_C|SetMaxHP _asbp_third_person_character (+ (Variables|/Game/ThirdPerson/Blueprints/BP_ThirdPersonCharacter.BP_ThirdPersonCharacter_C|GetMaxHP _asbp_third_person_character) 2e+01)))
    (Variables|/Game/ThirdPerson/Blueprints/BP_ThirdPersonCharacter.BP_ThirdPersonCharacter_C|SetHP _asbp_third_person_character _output_get)
    (bind _output_get_2 (Variables|/Game/ThirdPerson/Blueprints/BP_ThirdPersonCharacter.BP_ThirdPersonCharacter_C|SetMaxStamina _asbp_third_person_character (+ (Variables|/Game/ThirdPerson/Blueprints/BP_ThirdPersonCharacter.BP_ThirdPersonCharacter_C|GetMaxStamina _asbp_third_person_character) 4e+01)))
    (Variables|/Game/ThirdPerson/Blueprints/BP_ThirdPersonCharacter.BP_ThirdPersonCharacter_C|SetStamina _asbp_third_person_character _output_get_2)
    (Default|UpdateHUD _asbp_third_person_character)
    (Utilities|FlowControl|Delay (Variables|Default|GetOpenDelay))
    (Default|OpenDoor (Variables|Default|GetDoorToOpen))))

(event EventBeginPlay)

(event Collision|EventActorBeginOverlap
  (params (OtherActor :type Actor%20Object%20Reference)))

(event EventTick
  (params (DeltaSeconds :type Float%20%28single-precision%29)))

(fn ConstructionScript)