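; AI controller for enemies that chases or reacts to the player through perception.
; On possess it sets up the BB_Enemy blackboard and runs the BT_Enemy behavior tree.
; Perception updates write a sensed BP_ThirdPersonCharacter into the TargetActor key.
; Any lost-stimulus update clears that key, whichever actor it came from.
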(event OnTargetPerceptionUpdated(AIPerception)
  (params (Actor :type Actor%20Object%20Reference) (Stimulus :type AI%20Stimulus%20Structure))
  (bind _returnvalue (Utilities|String|StringToName "TargetActor"))
  (bind _bbref (Variables|Default|GetBBRef))
  (if (.bSuccessfullySensed (Utilities|Struct|BreakAIStimulus Stimulus))
    (bind _asbp_third_person_character (Utilities|Casting|CastToBP_ThirdPersonCharacter Actor))
    (AI|Components|Blackboard|SetValueasObject _bbref _returnvalue _asbp_third_person_character)
    (else
      (AI|Components|Blackboard|ClearValue _bbref _returnvalue))))

(event EventBeginPlay)

(event EventTick
  (params (DeltaSeconds :type Float%20%28single-precision%29)))

(event EventPossess
  (params (PossessedPawn :type Pawn%20Object%20Reference))
  (bind _blackboardcomponent (Class|AIController|UseBlackboard "/Game/_Project/03_characters/Enemies/AI/BlackBoards/BB_Enemy.BB_Enemy"))
  (Variables|Default|SetBBRef _blackboardcomponent)
  (AI|RunBehaviorTree "/Game/_Project/03_characters/Enemies/AI/BehaviorTrees/BT_Enemy.BT_Enemy"))

(fn ConstructionScript)