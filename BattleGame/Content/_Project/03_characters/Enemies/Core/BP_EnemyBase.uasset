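; BP_EnemyBase is a base enemy character that handles health and death.
; On BeginPlay it copies max HP, attack damage and walk speed from an EnemyConfig, when one is valid.
; AnyDamage reduces and prints HP, then at zero or below sets IsDead and calls Die.
; Die broadcasts OnDied, disables capsule collision and movement, stops any AI controller's movement and turns on mesh physics for a ragdoll.
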(event EventBeginPlay
  (if (Utilities|IsValid (Variables|Default|GetEnemyConfig))
    (bind _output_get (Variables|Default|SetMaxHP (Variables|/Game/_Project/07_Core/Data/DA_EnemyConfig.DA_EnemyConfig_C|GetMaxHP (Variables|Default|GetEnemyConfig))))
    (Variables|Default|SetHP _output_get)
    (Variables|Default|SetAttackDamage (Variables|/Game/_Project/07_Core/Data/DA_EnemyConfig.DA_EnemyConfig_C|GetAttackDamage (Variables|Default|GetEnemyConfig)))
    (Variables|/Script/Engine.CharacterMovementComponent|SetMaxWalkSpeed (Variables|Character|GetCharacterMovement) (Variables|/Game/_Project/07_Core/Data/DA_EnemyConfig.DA_EnemyConfig_C|GetWalkSpeed (Variables|Default|GetEnemyConfig)))))

(event Collision|EventActorBeginOverlap
  (params (OtherActor :type Actor%20Object%20Reference)))

(event EventTick
  (params (DeltaSeconds :type Float%20%28single-precision%29)))

(event Game|Damage|EventAnyDamage
  (params (Damage :type Float%20%28single-precision%29) (DamageType :type Damage%20Type%20Object%20Reference) (InstigatedBy :type Controller%20Object%20Reference) (DamageCauser :type Actor%20Object%20Reference))
  (bind _output_get (Variables|Default|SetHP (- (Variables|Default|GetHP) Damage)))
  (Development|PrintString (Utilities|String|ToString(Float) _output_get))
  (if (<= _output_get 0.0)
    (Variables|Default|SetisDead true)
    (CallFunction|Die)))

(fn ConstructionScript)

(fn Die
  (bind _charactermovement (Variables|Character|GetCharacterMovement))
  (if (Variables|Default|GetisDead)
    (Default|CallOnDied)
    (Collision|SetCollisionEnabled (Variables|Collision|GetCapsuleComponent) "NoCollision")
    (Pawn|Components|CharacterMovement|DisableMovement _charactermovement)
    (Components|Movement|StopMovementImmediately _charactermovement)
    (bind _asaicontroller (Utilities|Casting|CastToAIController (Pawn|GetController)))
    (AI|Navigation|StopMovement _asaicontroller)
    (Physics|SetSimulatePhysics (Variables|Character|GetMesh) true)))